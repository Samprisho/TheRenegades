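; Procedural arena floor built with Geometry Script as a grid of tall, spaced boxes on a dynamic mesh, with one animated top face.
; When Generate is set, the construction script appends the boxes, finds upward-facing polygroups, gives each a random height and builds collision.
; On BeginPlay, a looping timeline drives the vertex heights of the third stored polygroup, rebuilding collision every update.
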(event EventBeginPlay
  (bind _triangle_ids_out (Variables|Default|GetTriangle%20IDs%20Out))
  (bind _returnvalue (Class|GeometryScriptLibraryMeshPolygroupFunctions|GetTrianglesinPolygroup :TargetMesh (Variables|Default|GetMesh) :PolygroupID (Utilities|Array|Get(acopy) (Variables|Default|GetPolygroup%20Index%20Array) 2) :TriangleIDsOut _triangle_ids_out))
  (bind (_selection _returnvalue_2) (Class|GeometryScriptLibraryMeshSelectionFunctions|ConvertIndexListtoMeshSelection _returnvalue _triangle_ids_out "Vertices"))
  (bind _indexarray (Class|GeometryScriptLibraryMeshSelectionFunctions|ConvertMeshSelectiontoIndexArray _returnvalue_2 _selection))
  (bind _output_get (Variables|Default|SetFace _indexarray))
  (bind _newtrack_0 (Timeline|Timeline Play)
    (:Update
      (for _array_element _output_get
        (Class|GeometryScriptLibraryMeshBasicEditFunctions|SetVertexPosition (Variables|Default|GetMesh) _array_element (Math|Vector|MakeVector (.x (.ReturnValue (Class|GeometryScriptLibraryMeshQueryFunctions|GetVertexPosition (Variables|Default|GetMesh) _array_element))) (.y (.ReturnValue (Class|GeometryScriptLibraryMeshQueryFunctions|GetVertexPosition (Variables|Default|GetMesh) _array_element))) _newtrack_0) false))
      (Class|GeometryScriptLibraryCollisionFunctions|SetDynamicMeshCollisionfromMesh (Variables|Default|GetMesh) (Variables|Components|GetDynamicMesh) (Utilities|Struct|MakeGeometryScriptCollisionfromMeshOptions true "MinVolumeShapes" false true false 1.0 true 25 1 0.5 0.0 0.1 0.1 "Z" true 0) 0))
    (:Finished
      (Timeline|Timeline PlayFromStart))))

(fn ConstructionScript
  (bind _box_size (Variables|Default|GetBox%20Size))
  (bind _box_size_2 (Variables|Default|GetBox%20Size))
  (bind _spacing (Variables|Default|GetSpacing))
  (bind _box_size_3 (Variables|Default|GetBox%20Size))
  (bind _triangle_id (LocalVariables|GetTriangle%20ID))
  (bind _returnvalue (* _box_size 0.5))
  (bind _returnvalue_2 (+ _box_size_2 _spacing))
  (if (Variables|Default|GetGenerate?)
    (Utilities|Array|Clear (Variables|Default|GetPolygroup%20Index%20Array))
    (bind _returnvalue_3 (DynamicMeshComponent|GetDynamicMesh (Variables|Components|GetDynamicMesh)))
    (Variables|Default|SetMesh _returnvalue_3)
    (for _index (range 0 (Variables|Default|GetSteps%20Y))
      (LocalVariables|SetCurrent%20Y%20Step _index)
      (for _index_2 (range 0 (Variables|Default|GetSteps%20X))
        (LocalVariables|SetCurrent%20X%20Step _index_2)
        (Class|GeometryScriptLibraryMeshPrimitiveFunctions|AppendBox (Variables|Default|GetMesh) (Utilities|Struct|MakeGeometryScriptPrimitiveOptions "PerFace" false "Uniform") (Math|Transform|MakeTransform (Math|Vector|MakeVector (+ (* (LocalVariables|GetCurrent%20X%20Step) _returnvalue_2) _returnvalue) (+ _returnvalue (* (LocalVariables|GetCurrent%20Y%20Step) _returnvalue_2)) 0.0) "0, 0, 0" "1.000000,1.000000,1.000000") _box_size_3 _box_size_3 2e+03 0 0 0 "Center" 0)))
    (bind _returnvalue_4 (Class|GeometryScriptLibraryMeshPolygroupFunctions|ComputePolygroupsfromPolygonDetection :TargetMesh (Variables|Default|GetMesh) :Debug 0))
    (bind (_selection _returnvalue_5) (Class|GeometryScriptLibraryMeshSelectionFunctions|SelectMeshElementsbyNormalAngle _returnvalue_4 (Transformation|GetActorUpVector) 0.0 "Polygroups" false))
    (bind _indexarray (Class|GeometryScriptLibraryMeshSelectionFunctions|ConvertMeshSelectiontoIndexArray _returnvalue_5 _selection))
    (CallFunction|RemoveDuplicates _indexarray)
    (for _array_element (Variables|Default|GetPolygroup%20Index%20Array)
      (LocalVariables|SetFace%20height (Math|Random|RandomFloatinRange 0.0 5e+01))
      (bind _returnvalue_6 (Class|GeometryScriptLibraryMeshPolygroupFunctions|GetTrianglesinPolygroup :TargetMesh (Variables|Default|GetMesh) :PolygroupID _array_element :TriangleIDsOut _triangle_id))
      (bind (_selection_2 _returnvalue_7) (Class|GeometryScriptLibraryMeshSelectionFunctions|ConvertIndexListtoMeshSelection _returnvalue_6 _triangle_id "Vertices"))
      (bind (_indexarray_2 _selectiontype _returnvalue_8) (Class|GeometryScriptLibraryMeshSelectionFunctions|ConvertMeshSelectiontoIndexArray _returnvalue_7 _selection_2))
      (for _array_element_2 _indexarray_2
        (Class|GeometryScriptLibraryMeshBasicEditFunctions|SetVertexPosition _returnvalue_8 _array_element_2 (Math|Vector|MakeVector (.x (.ReturnValue (Class|GeometryScriptLibraryMeshQueryFunctions|GetVertexPosition _returnvalue_8 _array_element_2))) (.y (.ReturnValue (Class|GeometryScriptLibraryMeshQueryFunctions|GetVertexPosition _returnvalue_8 _array_element_2))) (LocalVariables|GetFace%20height)) false)))
    (Class|GeometryScriptLibraryCollisionFunctions|SetDynamicMeshCollisionfromMesh (Variables|Default|GetMesh) (Variables|Components|GetDynamicMesh) (Utilities|Struct|MakeGeometryScriptCollisionfromMeshOptions true "MinVolumeShapes" true true true 1.0 true 25 1 0.5 0.0 0.1 0.1 "Z" true 0) 0)))

(fn RemoveDuplicates
  (params (Array :type Array%20of%20Integers))
  (for _array_element Array
    (Utilities|Array|AddUnique (Variables|Default|GetPolygroup%20Index%20Array) _array_element)))