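; Base player character Blueprint that handles movement, sprinting and shooting input for a battle game.
; BeginPlay adds the weapons input mapping context for local player 0, then caches the owning battle controller.
; Enhanced Input drives move, jump and crouch, while a debug Z key toggles the sprint flag on the custom movement component while held.
; Shooting activates GA_Shoot through the Gameplay Ability System; the PlayerStateRep event is an empty stub.
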(event Input|EnhancedActionEvents|EnhancedInputActionIA_Move
  (params (ActionValue :type Vector%202D%20Structure) (ElapsedSeconds :type Float%20%28double-precision%29) (TriggeredSeconds :type Float%20%28double-precision%29) (InputAction :type Input%20Action%20Object%20Reference :default "/Game/Pre-madeAssets/FirstPerson/Input/Actions/IA_Move.IA_Move"))
  (Pawn|Input|AddMovementInput (Transformation|GetActorForwardVector) (.y ActionValue) false)
  (Pawn|Input|AddMovementInput (Transformation|GetActorRightVector) (.x ActionValue) false))

(event Input|EnhancedActionEvents|EnhancedInputActionIA_Jump
  (params (ActionValue :type Boolean) (ElapsedSeconds :type Float%20%28double-precision%29) (TriggeredSeconds :type Float%20%28double-precision%29) (InputAction :type Input%20Action%20Object%20Reference :default "/Game/Pre-madeAssets/FirstPerson/Input/Actions/IA_Jump.IA_Jump"))
  (:Triggered
    (Character|Jump))
  (:Completed
    (Character|StopJumping)))

(event Input|EnhancedActionEvents|EnhancedInputActionIA_Crouch
  (params (ActionValue :type Boolean) (ElapsedSeconds :type Float%20%28double-precision%29) (TriggeredSeconds :type Float%20%28double-precision%29) (InputAction :type Input%20Action%20Object%20Reference :default "/Game/Pre-madeAssets/FirstPerson/Input/Actions/IA_Crouch.IA_Crouch"))
  (:Triggered
    (Character|Crouch))
  (:Completed
    (Character|UnCrouch)))

(event Input|EnhancedActionEvents|EnhancedInputActionIA_Shoot
  (params (ActionValue :type Boolean) (ElapsedSeconds :type Float%20%28double-precision%29) (TriggeredSeconds :type Float%20%28double-precision%29) (InputAction :type Input%20Action%20Object%20Reference :default "/Game/Pre-madeAssets/FirstPerson/Input/Actions/IA_Shoot.IA_Shoot"))
  (Abilities|TryActivateAbilitybyClass (Ability|GetAbilitySystemComponent 0) "/Game/Blueprints/GameplayAbilities/GA_Shoot.GA_Shoot_C" true))

(event EventBeginPlay
  (bind _returnvalue (Game|GetPlayerController 0))
  (bind _returnvalue_2 (PlayerController|LocalPlayerSubsystems|GetEnhancedInputLocalPlayerSubsystem _returnvalue))
  (Utilities|IsValid _returnvalue_2
    (:Is%20Valid
      (Input|AddMappingContext _returnvalue_2 "/Game/Pre-madeAssets/FirstPerson/Input/IMC_Weapons.IMC_Weapons" 0 "(bIgnoreAllPressedKeysUntilRelease=True,bForceImmediately=False,bNotifyUserSettings=False)")
      (bind _asbp_base_battle_controller (Utilities|Casting|CastToBP_BaseBattleController (Pawn|GetController)))
      (Variables|Default|SetBattle%20Controller _asbp_base_battle_controller))))

(event EventPlayerStateRep)

(event Input|KeyboardEvents|DebugKeyZ
  (params (Key :type Key%20Structure :default "None") (ActionValue :type Input%20Action%20Value%20Structure))
  (bind _returnvalue (Class|PBBaseCharacter|GetCustomCharacterMovement))
  (:Pressed
    (Variables|/Script/TheRenegades.CustomPBPlayerMovement|SetbWantsToSprint _returnvalue true))
  (:Released
    (Variables|/Script/TheRenegades.CustomPBPlayerMovement|SetbWantsToSprint _returnvalue false)))

(fn ConstructionScript)