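; GC_BulletHit is a gameplay cue that plays a burst effect where a bullet hits.
; On execute, it skips the effect when the target is player 0's controlled pawn, so that player does not see it when hit.
; Otherwise, given a hit result, it spawns a pooled, auto-released Niagara burst at the hit location, oriented to the impact normal, then calls the parent implementation.
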(fn OnExecute
  (params (MyTarget :type Actor%20Object%20Reference) (Parameters :type Gameplay%20Cue%20Parameters%20Structure%20%28by%20ref%29))
  (bind _returnvalue (Ability|EffectContext|GetHitResult Parameters))
  (if (!= MyTarget (Pawn|GetControlledPawn (Game|GetPlayerController MyTarget))) ; Make sure target doesn't see vfx
    (if (Class|AbilitySystemBlueprintLibrary|HasHitResult Parameters)
      (Niagara|SpawnSystematLocation 0 "/Game/VFX/NS_Burst.NS_Burst" (.location _returnvalue) (Math|Rotator|MakeRotfromZ (.impactnormal _returnvalue)) "1.000000,1.000000,1.000000" true true "AutoRelease")
      (return (|CallParentFunction MyTarget Parameters)))))