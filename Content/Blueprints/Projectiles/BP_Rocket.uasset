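; Rocket projectile that launches nearby characters away from its impact point, with separate horizontal scaling for its instigator, and deals no damage.
; On stop it destroys itself and sphere-overlaps pawns, but client-created copies launch only their instigator, which suggests client-side prediction.
; A simulated proxy hides itself and skips the explosion when the local player is its instigator.
; Tick pulses the Trial mesh's Y scale with a fast sine wave.
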(event OnProjectileStop(ProjectileMovement)
  (params (ImpactResult :type Hit%20Result%20Structure%20%28by%20ref%29))
  (bind _launch_power (Variables|Default|GetLaunch%20Power))
  (if (not (Variables|Default|GetHidden))
    (Actor|DestroyActor)
    (bind (_outactors _returnvalue) (Collision|SphereOverlapActors (Transformation|GetActorLocation) (Variables|Default|GetExplosion%20Radius) (Utilities|Array|MakeArray "ObjectTypeQuery3") 0 (Utilities|Array|MakeArray self)))
    (if _returnvalue
      (for _array_element _outactors
        (if (not (Variables|Default|GetIsClientCreated?))
          (bind _ascharacter (Utilities|Casting|CastToCharacter _array_element :!label _label))
          (Character|LaunchCharacter _ascharacter (* (Math|Vector|GetUnitDirection(Vector) (Transformation|GetActorLocation) (Transformation|GetActorLocation _ascharacter)) (Math|Vector|MakeVector (* _launch_power (Math|Float|SelectFloat (Variables|Default|GetHorizantalLaunchMulti) 0.5 (== _ascharacter (Game|GetInstigator)))) (* _launch_power (Math|Float|SelectFloat (Variables|Default|GetHorizantalLaunchMulti) 0.5 (== _ascharacter (Game|GetInstigator)))) (* _launch_power (Variables|Default|GetVerticalLaunchMulti)))) false false)
          (elif (== _array_element (Game|GetInstigator))
            (goto _label)))))))

(event EventBeginPlay
  (Collision|IgnoreActorwhenMoving (Variables|Default|GetBox) (Variables|Actor|GetInstigator) true)
  (if (and (Utilities|Enum|Equal(Enum) (Networking|GetLocalRole) "ROLE_SimulatedProxy") (== (Game|GetInstigator) (Pawn|GetControlledPawn (Game|GetPlayerController 0))))
    (Rendering|SetActorHiddenInGame true)
    (Variables|Default|SetHidden true)
    (else
      (Utilities|IsValid self
        (:Is%20Valid
          (Variables|Default|SetStarting%20Scale (Variables|/Script/Engine.SceneComponent|GetRelativeScale3D (Variables|Default|GetTrial))))))))

(event EventTick
  (params (DeltaSeconds :type Float%20%28single-precision%29))
  (bind _starting_scale (Variables|Default|GetStarting%20Scale))
  (bind _returnvalue (* (.y _starting_scale) 0.5))
  (Utilities|IsValid self
    (:Is%20Valid
      (Transformation|SetRelativeScale3D (Variables|Default|GetTrial) (Math|Vector|MakeVector (.x _starting_scale) (Math|Float|Lerp (+ (.y _starting_scale) _returnvalue) (- (.y _starting_scale) _returnvalue) (Math|Float|Absolute(Float) (Math|Trig|Sin(Radians) (* (Utilities|Time|GetTimeSeconds) 5e+01)))) (.z _starting_scale))))))

(fn ConstructionScript
  (bind _projectilemovement (Variables|Default|GetProjectileMovement))
  (Game|Components|ProjectileMovement|Interpolation|SetInterpolatedComponent _projectilemovement (Variables|Default|GetBox))
  (Variables|/Script/Engine.ProjectileMovementComponent|SetInitialSpeed _projectilemovement (Variables|Default|GetInitial%20Speed))
  (Variables|Default|SetbNetUseOwnerRelevancy false))