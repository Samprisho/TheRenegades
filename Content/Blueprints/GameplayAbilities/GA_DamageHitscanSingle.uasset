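; Gameplay ability that deals single hitscan damage from the avatar's BP character.
; On activation it traces a very long line on the Visibility channel from the camera along control rotation, ignoring the character and drawing debug for one frame.
; A valid hit actor becomes target data for applying the GE_Damag gameplay effect.
; The graph has no commit or end-ability call.
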(event Ability|EventActivateAbility
  (bind _asbp_base_char (Utilities|AttemptGetBPCharfromAvatar)
    (:then
      (bind (_outhit _returnvalue) (Collision|LineTraceByChannel (Transformation|GetWorldLocation (Variables|/Game/Blueprints/BP_BaseChar.BP_BaseChar_C|GetCamera _asbp_base_char)) (+ (Transformation|GetWorldLocation (Variables|/Game/Blueprints/BP_BaseChar.BP_BaseChar_C|GetCamera _asbp_base_char)) (* (Math|Vector|GetForwardVector (Pawn|GetControlRotation _asbp_base_char :!class /Script/Engine.Pawn)) 2e+12)) "TraceTypeQuery1" true (Utilities|Array|MakeArray _asbp_base_char) "ForOneFrame"))
      (if _returnvalue
        (Utilities|IsValid (.HitActor (Collision|BreakHitResult _outhit))
          (:Is%20Valid
            (GameplayEffects|ApplyGameplayEffectToTarget (Ability|TargetData|AbilityTargetDatafromHitResult _outhit) "/Game/Blueprints/GameplayEffects/GE_Damag.GE_Damag_C" 1 1)))))))