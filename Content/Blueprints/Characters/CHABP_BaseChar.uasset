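; Base character Blueprint that turns Enhanced Input actions into basic movement: walking, jumping and crouching.
; The move action's 2D value feeds the Character Movement component as input vectors along the actor's forward and right axes.
; Crouch and jump start on their actions' Triggered events and end on Completed, and the construction script is empty.
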(event Input|EnhancedActionEvents|EnhancedInputActionIA_Jump
  (params (ActionValue :type Boolean) (ElapsedSeconds :type Float%20%28double-precision%29) (TriggeredSeconds :type Float%20%28double-precision%29) (InputAction :type Input%20Action%20Object%20Reference :default "/Game/Pre-madeAssets/FirstPerson/Input/Actions/IA_Jump.IA_Jump"))
  (:Triggered
    (Character|Jump))
  (:Completed
    (Character|StopJumping)))

(event Input|EnhancedActionEvents|EnhancedInputActionIA_Move
  (params (ActionValue :type Vector%202D%20Structure) (ElapsedSeconds :type Float%20%28double-precision%29) (TriggeredSeconds :type Float%20%28double-precision%29) (InputAction :type Input%20Action%20Object%20Reference :default "/Game/Pre-madeAssets/FirstPerson/Input/Actions/IA_Move.IA_Move"))
  (Class|PawnMovementComponent|AddInputVector (Variables|Character|GetCharacterMovement) (* (.y ActionValue) (Transformation|GetActorForwardVector)) false)
  (Class|PawnMovementComponent|AddInputVector (Variables|Character|GetCharacterMovement) (* (.x ActionValue) (Transformation|GetActorRightVector)) false))

(event Input|EnhancedActionEvents|EnhancedInputActionIA_Crouch
  (params (ActionValue :type Boolean) (ElapsedSeconds :type Float%20%28double-precision%29) (TriggeredSeconds :type Float%20%28double-precision%29) (InputAction :type Input%20Action%20Object%20Reference :default "/Game/Pre-madeAssets/FirstPerson/Input/Actions/IA_Crouch.IA_Crouch"))
  (:Triggered
    (Character|Crouch))
  (:Completed
    (Character|UnCrouch)))

(fn ConstructionScript)